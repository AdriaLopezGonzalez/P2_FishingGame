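; Light puzzle actor with a spotlight that lights up near the player and can cycle through a set of colors.
; Sphere overlaps with the third-person character switch the spotlight intensity on when entering and to zero when leaving.
; BeginPlay applies the first entry of the LightColor array.
; ChangeColor steps to the next entry and wraps to the start, with no caller inside this Blueprint.
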(event `self.ReceiveBeginPlay`
  (`LightComponent.SetLightColor` (`self.SpotLight`) (`|GetArrayItem` (`self.Light Color`)) true))

(event `self.Sphere.OnComponentBeginOverlap`
  (params (OverlappedComponent :type "PrimitiveComponent Object Reference") (OtherActor :type "Actor Object Reference") (OtherComp :type "PrimitiveComponent Object Reference") (OtherBodyIndex :type Integer) (bFromSweep :type Boolean) (SweepResult :type "HitResult Structure (by ref)"))
  (cast `/Game/ThirdPerson/Blueprints/BP_ThirdPersonCharacter` OtherActor)
  (`LightComponent.SetIntensity` (`self.SpotLight`) 8000.0))

(event `self.Sphere.OnComponentEndOverlap`
  (params (OverlappedComponent :type "PrimitiveComponent Object Reference") (OtherActor :type "Actor Object Reference") (OtherComp :type "PrimitiveComponent Object Reference") (OtherBodyIndex :type Integer))
  (cast `/Game/ThirdPerson/Blueprints/BP_ThirdPersonCharacter` OtherActor)
  (`LightComponent.SetIntensity` (`self.SpotLight`) 0.0))

(fn `Change color`
  (`/Engine/EditorBlueprintResources/StandardMacros.IncrementInt` (`self.Light index`)
    (:`  `
      (if (> (`self.Light index`) (- (`KismetArrayLibrary.Array_Length` (`self.Light Color`)) 1))
        (set `self.Light index` 0))
      (`LightComponent.SetLightColor` (`self.SpotLight`) (`|GetArrayItem` (`self.Light Color`) (`self.Light index`)) true))))

(fn `UserConstructionScript`)